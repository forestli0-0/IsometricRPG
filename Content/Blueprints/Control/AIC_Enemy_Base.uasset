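; Base AI controller for enemies that runs a behavior tree on possess and tracks a sensed target through AI perception.
; When a stimulus is sensed, it stores the actor as TargetActor in the blackboard and clears LastKnownLocation.
; When sensing is lost, it records the stored target's current position as LastKnownLocation and clears TargetActor.
; Each change prints a debug message in Chinese.
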(event EventPossess
  (params (PossessedPawn :type Pawn%20Object%20Reference))
  (AI|RunBehaviorTree (Variables|Default|GetBTAsset)))

(fn ConstructionScript)

(fn OnTargetPerceptionUpdated
  (params (Actor :type Actor%20Object%20Reference) (Stimulus :type AI%20Stimulus%20Structure))
  (bind _returnvalue (AI|GetBlackboard 0))
  (bind _targetactor (LocalVariables|GetTargetActor))
  (bind _lastknownlocation (LocalVariables|GetLastKnownLocation))
  (if (.bSuccessfullySensed (Utilities|Struct|BreakAIStimulus Stimulus))
    (AI|Components|Blackboard|SetValueasObject _returnvalue _targetactor Actor)
    (Development|PrintString "我看见你了")
    (AI|Components|Blackboard|ClearValue _returnvalue _lastknownlocation)
    (else
      (bind _asactor (Utilities|Casting|CastToActor (AI|Components|Blackboard|GetValueasObject _returnvalue _targetactor)))
      (AI|Components|Blackboard|SetValueasVector _returnvalue _lastknownlocation (Transformation|GetActorLocation _asactor))
      (Development|PrintString "不，我跟丢了")
      (AI|Components|Blackboard|ClearValue _returnvalue _targetactor))))