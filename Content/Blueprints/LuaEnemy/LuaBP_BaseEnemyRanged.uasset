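; Base Blueprint for a ranged enemy, bound to the Lua script module Enemy/BaseEnemy through GetModuleName.
; On BeginPlay it passes itself to the WBP_EnemyHealthBar in its HP widget component, printing an error if the cast fails.
; Each Tick it billboards the health bar on yaw only, turning it to face opposite the first player's camera yaw.
; The graph itself contains no ranged attack logic.
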(event EventTick
  (params (DeltaSeconds :type Float%20%28single-precision%29))
  (Transformation|SetWorldRotation (Variables|Default|GetHP) (Math|Rotator|MakeRotator 0.0 0.0 (+ (.Yaw (Math|Rotator|BreakRotator (Camera|GetCameraRotation (Variables|/Script/Engine.PlayerController|GetPlayerCameraManager (Game|GetPlayerController 0))))) 1.8e+02)) false false))

(event EventBeginPlay
  ;[0.02618 0.15 0.06135 0.5] 更新血条
  (bind _aswbp_enemy_health_bar (Utilities|Casting|CastToWBP_EnemyHealthBar (UserInterface|GetWidget (Variables|Default|GetHP)))
    (:then
      (Variables|/Game/UI/WBP_EnemyHealthBar.WBP_EnemyHealthBar_C|SetBP_Enemy _aswbp_enemy_health_bar self))
    (:CastFailed
      (Development|PrintString "Enemy：获取血条失败"))))

(fn ConstructionScript)

(fn GetModuleName
  (return "Enemy/BaseEnemy"))