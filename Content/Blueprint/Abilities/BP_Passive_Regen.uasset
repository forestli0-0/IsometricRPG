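; BP_Passive_Regen is a Gameplay Ability that gives its owning IsometricRPGCharacter health and mana regeneration.
; On activation it reads the HealthRegenRate and ManaRegenRate values from the character's attribute set.
; It passes each as a SetByCaller magnitude, tagged Data.Regen.Health or Data.Regen.Mana, into HPRegen and ManaRegen effect specs applied to the owner.
; The rates are captured once at activation, and the ability never calls EndAbility.
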(event Ability|EventActivateAbility
  (Development|PrintString "Hello")
  (bind _asisometric_rpgcharacter (Utilities|Casting|CastToIsometricRPGCharacter (Ability|GetAvatarActorfromActorInfo)))
  (bind _asisometric_rpgattribute_set_base (Utilities|Casting|CastToIsometricRPGAttributeSetBase (Class|IsometricRPGCharacter|GetAttributeSet _asisometric_rpgcharacter)))
  (Variables|Default|SetHealth%20Regen%20Rate (Variables|/Script/IsometricRPG.IsometricRPGAttributeSetBase|GetHealthRegenRate _asisometric_rpgattribute_set_base))
  (Variables|Default|SetMana%20Regen%20Rate (Variables|/Script/IsometricRPG.IsometricRPGAttributeSetBase|GetManaRegenRate _asisometric_rpgattribute_set_base))
  (bind _returnvalue (Ability|GameplayEffect|AssignTagSetbyCallerMagnitude (Ability|MakeOutgoingGameplayEffectSpec (Variables|Default|GetHP_Regen) (Math|Conversions|ToFloat(Integer) (Ability|GetAbilityLevel))) "(TagName=\"Data.Regen.Health\")" (.CurrentValue (Utilities|Struct|BreakGameplayAttributeData (Variables|Default|GetHealth%20Regen%20Rate)))))
  (Ability|ApplyGameplayEffectSpecToOwner _returnvalue)
  (bind _returnvalue_2 (Ability|GameplayEffect|AssignTagSetbyCallerMagnitude (Ability|MakeOutgoingGameplayEffectSpec (Variables|Default|GetMana_Regen) (Math|Conversions|ToFloat(Integer) (Ability|GetAbilityLevel))) "(TagName=\"Data.Regen.Mana\")" (.CurrentValue (Utilities|Struct|BreakGameplayAttributeData (Variables|Default|GetMana%20Regen%20Rate)))))
  (Ability|ApplyGameplayEffectSpecToOwner _returnvalue_2))