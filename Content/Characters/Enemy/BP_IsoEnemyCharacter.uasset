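; Isometric RPG enemy character that shows a health bar and passes AI perception to its controller.
; On BeginPlay it hands itself and its Ability System Component to the health bar widget and binds to the attribute set's health-changed event.
; That event updates the bar's fill ratio.
; Perception updates are forwarded to TS_EnemyAIController, falling back to AIC_Enemy_Base if that cast fails.
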(event OnTargetPerceptionUpdated(AIPerception)
  (params (Actor :type Actor%20Object%20Reference) (Stimulus :type AI%20Stimulus%20Structure))
  (bind _self self)
  (bind _returnvalue (AI|GetAIController _self))
  ;[0.15 0.15 0.15 0.5] 通知控制器，发送感知信息
  (bind _asts_enemy_aicontroller (Utilities|Casting|CastToTS_EnemyAIController _returnvalue)
    (:then
      (Default|OnPerceptionUpdated _asts_enemy_aicontroller Actor Stimulus))
    (:CastFailed
      (bind _asaic_enemy_base (Utilities|Casting|CastToAIC_Enemy_Base _returnvalue))
      (Default|OnTargetPerceptionUpdated _asaic_enemy_base Actor Stimulus))))

(event Custom|血量改变时
  (params (AttributeSet :type Isometric%20RPG%20Attribute%20Set%20Base%20Object%20Reference) (NewHealth :type Float%20%28single-precision%29))
  ;[0.02618 0.15 0.06135 0.5] 更新血条
  (bind _aswbp_enemy_health_bar (Utilities|Casting|CastToWBP_EnemyHealthBar (UserInterface|GetWidget (Variables|Default|GetHealthBar))))
  (Progress|SetPercent (Variables|/Game/UI/WBP_EnemyHealthBar.WBP_EnemyHealthBar_C|GetProgressBar_98 _aswbp_enemy_health_bar) (/ NewHealth (.ReturnValue (Class|AbilitySystemComponent|GetGameplayAttributeValue (Ability|GetAbilitySystemComponent 0) "(AttributeName=\"MaxHealth\",Attribute=/Script/IsometricRPG.IsometricRPGAttributeSetBase:MaxHealth,AttributeOwner=\"/Script/CoreUObject.Class'/Script/IsometricRPG.IsometricRPGAttributeSetBase'\")")))))

(event EventBeginPlay
  (bind _returnvalue (Ability|GetAbilitySystemComponent 0))
  (bind _aswbp_enemy_health_bar (Utilities|Casting|CastToWBP_EnemyHealthBar (UserInterface|GetWidget (Variables|Default|GetHealthBar))))
  (Variables|/Game/UI/WBP_EnemyHealthBar.WBP_EnemyHealthBar_C|SetBP_Enemy _aswbp_enemy_health_bar self)
  (Variables|/Game/UI/WBP_EnemyHealthBar.WBP_EnemyHealthBar_C|SetASC _aswbp_enemy_health_bar _returnvalue)
  (bind _returnvalue_2 (GameplayAttributes|GetAttributeSet _returnvalue "/Script/IsometricRPG.IsometricRPGAttributeSetBase"))
  ;[0.02618 0.15 0.06135 0.5] 更新血条
  (bind _output_get (Variables|Default|SetMyAttributeSet _returnvalue_2))
  (EventDispatchers|BindEventtoOnHealthChanged _output_get (delegate Custom|血量改变时)))

(fn ConstructionScript)