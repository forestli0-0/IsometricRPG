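; Ranged enemy character that shows a health bar widget and relays what it senses to its AI controller.
; On BeginPlay it gives the widget itself and its Ability System Component, then binds to the attribute set's health-change event.
; Each change sets the bar's percent from new health over a gameplay attribute value.
; Perception updates forward to AIC_Enemy_Ranged; a separate auto-generated function only prints a debug string.
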(event OnTargetPerceptionUpdated(AIPerception)
  (params (Actor :type Actor%20Object%20Reference) (Stimulus :type AI%20Stimulus%20Structure))
  (bind _asaic_enemy_ranged (Utilities|Casting|CastToAIC_Enemy_Ranged (AI|GetAIController self)))
  (Default|OnTargetPerceptionUpdated _asaic_enemy_ranged Actor Stimulus))

(event Custom|自定义事件
  (params (AttributeSet :type Isometric%20RPG%20Attribute%20Set%20Base%20Object%20Reference) (NewHealth :type Float%20%28single-precision%29))
  ;[0.02618 0.15 0.06135 0.5] 更新血条
  (bind _aswbp_enemy_health_bar (Utilities|Casting|CastToWBP_EnemyHealthBar (UserInterface|GetWidget (Variables|Default|GetHealthBarWidget))))
  (Progress|SetPercent (Variables|/Game/UI/WBP_EnemyHealthBar.WBP_EnemyHealthBar_C|GetProgressBar_98 _aswbp_enemy_health_bar) (/ NewHealth (.ReturnValue (Class|AbilitySystemComponent|GetGameplayAttributeValue (Variables|Default|GetAbilitySystemComponent) "(AttributeName=\"MaxHealth\",Attribute=/Script/IsometricRPG.IsometricRPGAttributeSetBase:MaxHealth,AttributeOwner=\"/Script/CoreUObject.Class'/Script/IsometricRPG.IsometricRPGAttributeSetBase'\")")))))

(event EventBeginPlay
  (bind _aswbp_enemy_health_bar (Utilities|Casting|CastToWBP_EnemyHealthBar (UserInterface|GetWidget (Variables|Default|GetHealthBarWidget))))
  (Variables|/Game/UI/WBP_EnemyHealthBar.WBP_EnemyHealthBar_C|SetBP_Enemy _aswbp_enemy_health_bar self)
  (Variables|/Game/UI/WBP_EnemyHealthBar.WBP_EnemyHealthBar_C|SetASC _aswbp_enemy_health_bar (Variables|Default|GetAbilitySystemComponent))
  (bind _returnvalue (GameplayAttributes|GetAttributeSet (Variables|Default|GetAbilitySystemComponent) "/Script/IsometricRPG.IsometricRPGAttributeSetBase"))
  (bind _output_get (Variables|Default|SetMyAttributeSet _returnvalue))
  ;[0.02618 0.15 0.06135 0.5] 更新血条
  (EventDispatchers|BindEventtoOnHealthChanged _output_get (delegate Custom|自定义事件)))

(fn ConstructionScript)

(fn BPIsometricRPGEnemyCharacterAutoGenFunc
  (params (Health :type Float%20%28single-precision%29))
  (Development|PrintString "这样行吗"))